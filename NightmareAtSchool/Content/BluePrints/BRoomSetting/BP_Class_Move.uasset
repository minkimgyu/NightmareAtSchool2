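; BP_Class_Move is a test-style trigger Blueprint that reports reaching a location to the quest system.
; OnTriggered prints a debug message and calls CallCallQuest on GameEventPostOfficeSubsystem with a ReachLocation event for "TestZone".
; BeginPlay only prints a debug message.
; A MoveTimeline that would nudge TargetActor along X is never run, so nothing moves despite the name.
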(event `self.ReceiveTick`
  (params (DeltaSeconds :type "Float (single-precision)")))

(event `self.ReceiveActorBeginOverlap`
  (params (OtherActor :type "Actor Object Reference")))

(event `self.ReceiveBeginPlay`
  (`KismetSystemLibrary.PrintString` "Begin"))

(event `self.OnTriggered`
  (`KismetSystemLibrary.PrintString` "Hello")
  (`GameEventPostOfficeSubsystem.CallQuest` (subsystem `GameEventPostOfficeSubsystem`) "ReachLocation" "TestZone" 1))

(fn `UserConstructionScript`)