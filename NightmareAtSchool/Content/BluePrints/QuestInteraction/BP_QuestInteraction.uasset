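; BP_QuestInteraction is a quest trigger actor that reports quest progress when the player reaches it.
; On the first overlap by a Player-tagged actor, it sends the current quest type, target and amount through GameEventPostOfficeSubsystem.
; It then passes NextQuestID to BP_PlayerCharacter's item interaction call.
; A DoOnce with no reset makes this one-shot, and debug strings print on overlaps.
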(event `self.ReceiveActorBeginOverlap`
  (params (OtherActor :type "Actor Object Reference"))
  (if (`self.ActorHasTag` OtherActor "Player")
    (`KismetSystemLibrary.PrintString` (`KismetSystemLibrary.GetDisplayName` OtherActor))
    (`/Engine/EditorBlueprintResources/StandardMacros.DoOnce` false
      (:`Completed`
        (`GameEventPostOfficeSubsystem.CallQuest` (subsystem `GameEventPostOfficeSubsystem`) (`self.CurrentQuestType`) (`self.CurrentQuestTargetID`) (`self.CurrentQuestAmount`))
        (bind _asbp_player_character (cast `/Game/BluePrints/BP_PlayerCharacter` (`GameplayStatics.GetPlayerCharacter` 0)))
        (`/Game/BluePrints/BP_PlayerCharacter.OnItemInteration` _asbp_player_character (`self.NextQuestID`))))
    (else
      (`KismetSystemLibrary.PrintString` "퀘스트 지역 도달 못 함"))))

(fn `UserConstructionScript`)