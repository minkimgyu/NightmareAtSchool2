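; BP_Fog is a damaging fog volume that hurts the player while they stay inside it.
; On overlap by a Player-tagged actor it stores that actor and starts a looping timer, which applies damage each interval while the fog is active.
; Leaving clears the timer and player reference.
; The InactiveFog function switches off damage and hides the fog in game.
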(event `self.ReceiveActorBeginOverlap`
  (params (OtherActor :type "Actor Object Reference"))
  (if (`self.ActorHasTag` OtherActor "Player")
    (set `self.PlayerActor` OtherActor)
    (set `self.bIsInside` true)
    (bind _returnvalue (`KismetSystemLibrary.K2_SetTimerDelegate` (delegate `TakeDamage`) (`self.DamageInterval`) true))
    (set `self.TimerHandle` _returnvalue)))

(event `TakeDamage`
  (if (`self.bActive`)
    (`GameplayStatics.ApplyDamage` (`self.PlayerActor`) (`self.Damage`))))

(event `self.ReceiveActorEndOverlap`
  (params (OtherActor :type "Actor Object Reference"))
  (if (`self.ActorHasTag` OtherActor "Player")
    (set `self.PlayerActor` null)
    (set `self.bIsInside` false)
    (`KismetSystemLibrary.K2_ClearAndInvalidateTimerHandle` (`self.TimerHandle`))))

(fn `InactiveFog`
  (set `self.bActive` false)
  (`self.SetActorHiddenInGame` true))

(fn `UserConstructionScript`)