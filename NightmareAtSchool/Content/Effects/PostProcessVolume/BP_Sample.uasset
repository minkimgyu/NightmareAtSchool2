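; Sample Blueprint that maps an HP variable to damage screen-effect parameters in the MPC_Damaged material parameter collection.
; The Construction Script rescales HP against 100 and clamps each result, raising opacity, vignette, hallucination and pixel strength as HP falls while shrinking PixelScale.
; Values are written only on construction, as the event graph holds just disabled placeholder events, so runtime HP changes are not tracked here.
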(fn `UserConstructionScript`
  (bind _hp (`self.HP`))
  (`KismetMaterialLibrary.SetScalarParameterValue` "/Game/Effects/PostProcessVolume/MPC_Damaged.MPC_Damaged" "Full_Opacity" (`KismetMathLibrary.FClamp` (/ (- 100.0 _hp) 100.0)))
  (`KismetMaterialLibrary.SetScalarParameterValue` "/Game/Effects/PostProcessVolume/MPC_Damaged.MPC_Damaged" "HallucinationStrength" (`KismetMathLibrary.FClamp` (/ (- 1.0 (/ _hp 100.0)) 3.0) 0.0 0.3))
  (`KismetMaterialLibrary.SetScalarParameterValue` "/Game/Effects/PostProcessVolume/MPC_Damaged.MPC_Damaged" "HallucinationTimeSpeed" (`KismetMathLibrary.FClamp` (- 3.0 (* (/ _hp 100.0) 3.0)) 0.0 3.0))
  (`KismetMaterialLibrary.SetScalarParameterValue` "/Game/Effects/PostProcessVolume/MPC_Damaged.MPC_Damaged" "PixelScale" (`KismetMathLibrary.FClamp` (* (/ _hp 100.0) 500.0) 50.0 500.0))
  (`KismetMaterialLibrary.SetScalarParameterValue` "/Game/Effects/PostProcessVolume/MPC_Damaged.MPC_Damaged" "PixelStrength" (`KismetMathLibrary.FClamp` (- 1.0 (/ _hp 100.0))))
  (`KismetMaterialLibrary.SetScalarParameterValue` "/Game/Effects/PostProcessVolume/MPC_Damaged.MPC_Damaged" "Vignette_Opacity" (`KismetMathLibrary.FClamp` (- 1.0 (/ _hp 100.0)) 0.0 1.0)))